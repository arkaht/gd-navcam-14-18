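; Wounded NPC Blueprint that the player can heal by interacting while carrying a medkit.
; The NPC crouches on BeginPlay to show it is wounded.
; CanInteract requires both the wounded flag and a player medkit.
; On interaction it consumes the medkit, clears the wounded flag, then stands up after a short delay.
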(event OnInteract(BPAC_Interactable)
  (params (Player :type BPC%20Player%20Object%20Reference))
  (Default|ConsumeMedkit Player)
  (Variables|Default|SetIs%20Wounded false)
  (Utilities|FlowControl|Delay 1.0)
  (Character|UnCrouch))

(event EventBeginPlay
  (Character|Crouch))

(fn ConstructionScript)

(fn CanInteract
  (params (Player :type BPC%20Player%20Object%20Reference))
  (return (and (Variables|/Game/Programming/Core/BPC_Player.BPC_Player_C|GetHas%20Medkit Player) (Variables|Default|GetIs%20Wounded))))