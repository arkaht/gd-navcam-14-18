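; Interactable nurse NPC that guides the player through a scripted medkit-and-heal sequence gating a locked door.
; On BeginPlay it locks the door, binds heal and table-medkit destruction events, and calls the player after a delay.
; A state machine driven by those events shows dialog assets, asking for healing, then unlocking the door on another medkit destruction.
; Talking is only offered while calling, and moves the nurse to waiting.
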(event OnInteract(BPAC_Interactable)
  (params (Player :type BPC%20Player%20Object%20Reference))
  (switch Utilities|FlowControl|Switch|SwitchonE_NPCState_Nurse (Variables|Default|GetState)
    (:NewEnumerator1
      (Default|ShowDialogsAsset Player "/Game/Design/Data/Dialogs/DA_Dialog_Nurse_WaitForMedkit.DA_Dialog_Nurse_WaitForMedkit")
      (Variables|Default|SetState "NewEnumerator0"))))

(event Custom|On%20Medkit%20Destroyed
  (params (DestroyedActor :type Actor%20Object%20Reference))
  (bind _player (Variables|Default|GetPlayer))
  (switch Utilities|FlowControl|Switch|SwitchonE_NPCState_Nurse (Variables|Default|GetState)
    (:NewEnumerator1
      (Default|ShowDialogsAsset _player "/Game/Design/Data/Dialogs/DA_Dialog_Nurse_AskToHeal.DA_Dialog_Nurse_AskToHeal" :!label _label)
      (Variables|Default|SetState "NewEnumerator3"))
    (:NewEnumerator0
      (goto _label))
    (:NewEnumerator2
      (Default|ShowDialogsAsset _player "/Game/Design/Data/Dialogs/DA_Dialog_Nurse_Go.DA_Dialog_Nurse_Go")
      (Variables|/Game/Programming/GPE/Interactable/BPA_Door.BPA_Door_C|SetIs%20Locked (Variables|Default|GetLocking%20Door) false))))

(event Custom|On%20NPC%20Heal
  (Default|ShowDialogsAsset (Variables|Default|GetPlayer) "/Game/Design/Data/Dialogs/DA_Dialog_Nurse_AskToGoOut.DA_Dialog_Nurse_AskToGoOut")
  (Variables|Default|SetState "NewEnumerator2"))

(event EventBeginPlay
  (EventDispatchers|AssignOnHeal (Variables|Default|GetTo%20Heal%20NPC) (delegate Custom|On%20NPC%20Heal))
  (Variables|/Game/Programming/GPE/Interactable/BPA_Door.BPA_Door_C|SetIs%20Locked (Variables|Default|GetLocking%20Door) true)
  (for _array_element (Variables|Default|GetTable%20Medkits)
    (Game|AssignOnDestroyed _array_element (delegate Custom|On%20Medkit%20Destroyed)))
  ;[1 1 1 0.33] Show Start Dialog
  (Utilities|FlowControl|Delay 2.0)
  (bind _asbpc_player (Utilities|Casting|CastToBPC_Player (Game|GetPlayerCharacter 0)))
  (bind _output_get (Variables|Default|SetPlayer _asbpc_player))
  (Default|ShowDialogsAsset _output_get "/Game/Design/Data/Dialogs/DA_Dialog_Nurse_Calling.DA_Dialog_Nurse_Calling"))

(fn ConstructionScript)

(fn CanInteract
  (params (Player :type BPC%20Player%20Object%20Reference))
  (switch Utilities|FlowControl|Switch|SwitchonE_NPCState_Nurse (Variables|Default|GetState)
    (:NewEnumerator1
      (return true))))

(fn GetIcon
  (return "/Game/Art/Sprites/SPR_Icon_Talk.SPR_Icon_Talk"))