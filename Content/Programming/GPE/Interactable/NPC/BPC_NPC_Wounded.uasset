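; Wounded NPC character that the player can interact with to heal using a medkit.
; It starts crouched and offers a heal icon only while wounded and the player carries a medkit.
; On interaction it consumes the medkit, swaps a mesh material, fires its heal callback, plays a heal sound and dialog, then stands up after a short delay.
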(event OnInteract(BPAC_Interactable)
  (params (Player :type BPC%20Player%20Object%20Reference))
  (Default|ConsumeMedkit Player)
  (Variables|Default|SetIs%20Wounded false)
  (Rendering|Material|SetMaterial (Variables|Character|GetMesh) 1 "/Game/Characters/Mannequins/Materials/Instances/Manny/MI_Manny_02.MI_Manny_02")
  (Default|CallOnHeal)
  (CallFunction|PlaySoundDataonActor self "/Game/Design/Sounds/Interaction/DA_SoundData_Heal.DA_SoundData_Heal")
  (Default|ShowDialogsAsset Player (Variables|Default|GetHeal%20Dialog))
  (Utilities|FlowControl|Delay 1.0)
  (Character|UnCrouch))

(event EventBeginPlay
  (Character|Crouch))

(fn ConstructionScript)

(fn CanInteract
  (params (Player :type BPC%20Player%20Object%20Reference))
  (return (and (Variables|/Game/Programming/Core/BPC_Player.BPC_Player_C|GetHas%20Medkit Player) (Variables|Default|GetIs%20Wounded))))

(fn GetIcon
  (return "/Game/Art/Sprites/SPR_Icon_Heal.SPR_Icon_Heal"))